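; BP_Push is a Blueprint that recolors its PC component when the Honk input is pressed and holds a function for reducing a Patience value.
; Each press prints a debug string, creates a new dynamic instance of material M_1 on PC and sets its Color parameter to a random RGB value.
; SetPatience subtracts damage from Patience, clamped between zero and MaxPatience, unless PlayerInvencible is set.
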(event `InputAction|Honk`
  (params (Key :type "Key Structure"))
  (:`Pressed`
    (`KismetSystemLibrary.PrintString` "Space_Pushed")
    (bind _returnvalue (`PrimitiveComponent.CreateDynamicMaterialInstance` (`self.P_C`) 0 "/Game/MidtermBP/M_1.M_1" "None"))
    (`MaterialInstanceDynamic.SetVectorParameterValue` _returnvalue "Color" (`KismetMathLibrary.MakeColor` (`KismetMathLibrary.RandomFloatInRange` 0.0 1.0) (`KismetMathLibrary.RandomFloatInRange` 0.0 1.0) (`KismetMathLibrary.RandomFloatInRange` 0.0 1.0)))))

(fn `SetPatience`
  (params (Damage :type "Float (double-precision)"))
  (if (not (`self.PlayerInvencible`))
    (set `self.Patience` (`KismetMathLibrary.FClamp` (- (`self.Patience`) Damage) 0.0 (`self.MaxPatience`)))))

(fn `UserConstructionScript`)