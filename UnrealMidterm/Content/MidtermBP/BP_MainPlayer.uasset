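; Player Blueprint for a honk-timing game where honking at the wrong moment drains patience.
; Honk input toggles Honk/Mute sound mixes, while the HonkTrue timeline, played on BeginPlay and release, sets the WrongHonk flag.
; Wrong honks damage patience unless invincible and make other and rhythm cars honk back; right honks randomly recolor a dynamic material.
; Empty patience silences honking and shows the game-over widget with UI-only input.
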(event `InputAction|Honk`
  (params (Key :type "Key Structure"))
  ;[1 1 1] Honk_Mute_Unmute
  (:`Pressed`
    (`GameplayStatics.SetBaseSoundMix` "/Game/Sound/Honk.Honk")
    (`KismetSystemLibrary.PrintString` "honk")
    (`SkeletalMeshComponent.PlayAnimation` (`self.car3`) "/Game/Cars/car3_Anim.car3_Anim" false)
    (if (`self.WrongHonk`)
      (`KismetSystemLibrary.PrintString` "Wrong_Honk_Damge")
      (`self.UpdatePatience` (`self.Damage`))
      (`|ExecutionSequence`
        (:`then_0`
          (bind _outactors (`GameplayStatics.GetAllActorsOfClass` "/Game/Cars/OtherCar_BP.OtherCar_BP_C"))
          (for _array_element _outactors
            (`/Game/Cars/OtherCar_BP.Honk` _array_element)))
        (:`then_1`
          (bind _outactors_2 (`GameplayStatics.GetAllActorsOfClass` "/Game/Cars/RhythmCar1_BP.RhythmCar1_BP_C"))
          (`/Game/Cars/RhythmCar1_BP.Honk` (`|GetArrayItem` _outactors_2)))
        (:`then_2`
          (bind _outactors_3 (`GameplayStatics.GetAllActorsOfClass` "/Game/Cars/RhythmCar2_BP.RhythmCar2_BP_C"))
          (`/Game/Cars/RhythmCar2_BP.Honk` (`|GetArrayItem` _outactors_3))))
      (else
        ;[1 1 1] Right_Honk
        (`KismetSystemLibrary.PrintString` "No_Damage")
        (bind _returnvalue (`PrimitiveComponent.CreateDynamicMaterialInstance` (`self.P_C`) 0 "/Game/MidtermBP/M_1.M_1" "None"))
        (`MaterialInstanceDynamic.SetVectorParameterValue` _returnvalue "Color" (`KismetMathLibrary.MakeColor` (`KismetMathLibrary.RandomFloatInRange` 0.0 1.0) (`KismetMathLibrary.RandomFloatInRange` 0.0 1.0) (`KismetMathLibrary.RandomFloatInRange` 0.0 1.0))))))
  (:`Released`
    (`GameplayStatics.SetBaseSoundMix` "/Game/Sound/Mute.Mute" :!label _label)
    ;[1 1 1] Time_Line(Right and Wrong Honk)
    (bind (_direction _one_zero) (`Timeline|HonkTrue`)
      (:`Update`
        (switch `int` (`KismetMathLibrary.FFloor` _one_zero)
          (:`0`
            (set `self.WrongHonk` true))
          (:`1`
            (set `self.WrongHonk` false)))))))

(event `self.ReceiveBeginPlay`
  ;[1 1 1] Time_Line(Right and Wrong Honk)
  (goto _label))

(event `self.ReceiveTick`
  (params (DeltaSeconds :type "Float (single-precision)")))

(fn `GameOver`
  (bind _returnvalue (`GameplayStatics.GetPlayerController` 0))
  (`GameplayStatics.SetSoundMixClassOverride` "/Game/Sound/Honk.Honk" "/Game/Sound/Honk_Class.Honk_Class" 0.0 1.0 0.0) ; Rong: It should be close, but dont know how to do
  (bind _returnvalue_2 (`|CreateWidget` "/Game/MidtermBP/BPW_GameOver.BPW_GameOver_C"))
  (`UserWidget.AddToViewport` _returnvalue_2 0)
  (set `PlayerController.bShowMouseCursor` true _returnvalue)
  (`WidgetBlueprintLibrary.SetInputMode_UIOnlyEx` _returnvalue _returnvalue_2))

(fn `OtherCarsHonk`)

(fn `UpdatePatience`
  (params (Damage :type "Float (double-precision)"))
  (if (not (`self.PlayerInvencible`))
    (bind _output_get (set `self.Patience` (`KismetMathLibrary.FClamp` (- (`self.Patience`) Damage) 0.0 (`self.MaxPatience`))))
    (if (<= _output_get 0.0)
      (`self.GameOver`))))

(fn `UserConstructionScript`)